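; Player-controlled physics spaceship with throttle, pitch, yaw, roll and a held super-speed boost.
; Rotation axes apply acceleration-based torque around the ship's own axes.
; Throttle input eases Thrust toward a target that boost greatly raises via a smaller lerp divisor, and holds it near zero input.
; Tick overwrites linear velocity with forward thrust plus a vertical term computed below the Gravity speed threshold and eased out above it.
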(event `self.ReceiveBeginPlay`
  ;[1 1 1] Thrust
  (set `self.thrust` 0.0))

(event `InputAction|super`
  (params (Key :type "Key Structure"))
  ;[1 1 1] Thrust Input
  (:`Pressed`
    (bind _output_get (set `self.superspeed` true)))
  (:`Released`
    (set `self.superspeed` false)))

(event `InputAxis|MoveUp`
  (params (AxisValue :type "Float (single-precision)"))
  ;[1 1 1] MoveUP
  (`PrimitiveComponent.AddTorqueInDegrees` (`self.ship`) (* (`SceneComponent.GetRightVector` (`self.ship`)) (* AxisValue (`self.forwardpower`))) "None" true))

(event `InputAxis|Thrust`
  (params (AxisValue :type "Float (single-precision)"))
  ;[1 1 1] Thrust Input
  (`|ExecutionSequence`
    (:`then_0`
      (if (stale `InputAction|super` _output_get)
        (if (not (`KismetMathLibrary.NearlyEqual_FloatFloat` AxisValue 0.0 0.1))
          (set `self.thrust` (`KismetMathLibrary.FInterpTo` (`self.thrust`) (`KismetMathLibrary.Lerp` 0.0 (`self.maxthrust`) (/ (+ AxisValue 1.0) 0.1)) (`GameplayStatics.GetWorldDeltaSeconds`) 5.0)))
        (elif (not (`KismetMathLibrary.NearlyEqual_FloatFloat` AxisValue 0.0 0.1))
          (set `self.thrust` (`KismetMathLibrary.FInterpTo` (`self.thrust`) (`KismetMathLibrary.Lerp` 0.0 (`self.maxthrust`) (/ (+ AxisValue 1.0) 2.0)) (`GameplayStatics.GetWorldDeltaSeconds`) 5.0)))))
    (:`then_1`
      (set `self.forward v` (* (`SceneComponent.GetForwardVector` (`self.ship`)) (`self.thrust`))))))

(event `InputAxis|MoveRight`
  (params (AxisValue :type "Float (single-precision)"))
  ;[1 1 1] MoveRight
  (`PrimitiveComponent.AddTorqueInDegrees` (`self.ship`) (* (`SceneComponent.GetUpVector` (`self.ship`)) (* AxisValue (`self.forwardpower`))) "None" true))

(event `self.ReceiveTick`
  (params (DeltaSeconds :type "Float (single-precision)"))
  ;[1 1 1] Event
  (`|ExecutionSequence`
    (:`then_0`
      (if (< (`KismetMathLibrary.VSize` (`self.forward v`)) (`self.gravity `))
        (set `self.upward v` (* (`KismetMathLibrary.Lerp` 0.0 -980.0 (- (`KismetMathLibrary.VSize` (`self.forward v`)) (`self.gravity `))) (`KismetMathLibrary.LessLess_VectorRotator` (`SceneComponent.GetUpVector` (`self.ship`)) (`SceneComponent.K2_GetComponentRotation` (`self.ship`)))))
        (else
          (set `self.upward v` (`KismetMathLibrary.VInterpTo` (`self.upward v`) (0.0 0.0 0.0) (`GameplayStatics.GetWorldDeltaSeconds`) 20.0)))))
    (:`then_1`
      (`PrimitiveComponent.SetPhysicsLinearVelocity` (`self.ship`) (+ (`self.forward v`) (`self.upward v`)) false "None"))))

(event `InputAxis|Roll`
  (params (AxisValue :type "Float (single-precision)"))
  ;[1 1 1] Roll
  (`PrimitiveComponent.AddTorqueInDegrees` (`self.ship`) (* (`SceneComponent.GetForwardVector` (`self.ship`)) (* AxisValue (`self.forwardpower`))) "None" true))

(fn `UserConstructionScript`)