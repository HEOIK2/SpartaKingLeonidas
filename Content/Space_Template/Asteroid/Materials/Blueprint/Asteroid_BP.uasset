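; Asteroid_BP builds an asteroid ring from instanced meshes and slowly spins it around its local Z axis on Tick.
; The construction script configures a hierarchical instanced mesh component's mesh and cull distances, then fills a length-by-width grid.
; The Asteroid function wraps each cell around the ring radius, adding random-stream position jitter and blending tangent-aligned rotation toward random.
; Instance scale grows with width index rather than being random.
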(event `self.ReceiveTick`
  (params (DeltaSeconds :type "Float (single-precision)"))
  (`self.K2_AddActorLocalRotation` (`KismetMathLibrary.RotatorFromAxisAndAngle` (0.0 0.0 1.0) (* DeltaSeconds (`self.rotationspeed`)))))

(fn `asteroid`
  (params (indexfromwidth :type Integer) (numberofinstancesbywidth :type Integer) (indexfromlegnth :type Integer) (numberofinstancesbylegnth :type Integer))
  (returns (outlocation :type "Vector Structure") (outrotating :type "Rotator Structure"))
  (bind _returnvalue (`KismetMathLibrary.MakeVector` 0.0 0.0 1.0))
  (bind _transfomrandm (`self.transfomrandm`))
  (bind _returnvalue_2 (`KismetMathLibrary.RotateAngleAxis` (+ (+ (* (- (`KismetMathLibrary.RandomFloatFromStream` _transfomrandm) 0.5) (`self.randomizezaxisposition`) (`self.ringwidth`)) (* (`KismetMathLibrary.RandomUnitVectorFromStream` _transfomrandm) (`self.randomizdposition`))) (`KismetMathLibrary.MakeVector` 0.0 (+ (`self.ringradius`) (* (- (/ (`KismetMathLibrary.Conv_IntToDouble` indexfromwidth) (`KismetMathLibrary.Conv_IntToDouble` numberofinstancesbywidth)) 0.5) (`self.ringwidth`))))) (* (/ (`KismetMathLibrary.Conv_IntToDouble` indexfromlegnth) (`KismetMathLibrary.Conv_IntToDouble` numberofinstancesbylegnth)) 360.0) _returnvalue))
  (return _returnvalue_2 (`KismetMathLibrary.RLerp` (`KismetMathLibrary.MakeRotFromYZ` (`KismetMathLibrary.Cross_VectorVector` _returnvalue _returnvalue_2) _returnvalue) (`KismetMathLibrary.RandomRotatorFromStream` (`self.transfomrandm`) true) (`self.randomizerotation`) true)))

(fn `UserConstructionScript`
  (bind _hierarchicalinstancedspawn (`self.HierarchicalInstancedSpawn`))
  (bind _instancecountbylenght (`self.instancecountbylenght`))
  (bind _instancecountbywidth (`self.instancecountbywidth`))
  (`|ExecutionSequence`
    (:`then_0`
      (`StaticMeshComponent.SetStaticMesh` _hierarchicalinstancedspawn (`self.instancemesh`)))
    (:`then_1`
      (`InstancedStaticMeshComponent.SetCullDistances` _hierarchicalinstancedspawn (`self.cullingnear`) (`self.cullingfaf`)))
    (:`then_2`
      (for _index (range _instancecountbylenght)
        (for _index_2 (range _instancecountbywidth)
          (bind (_outlocation _outrotating) (`self.asteroid` _index_2 _instancecountbywidth _index _instancecountbylenght))
          (`InstancedStaticMeshComponent.AddInstance` (`self.HierarchicalInstancedSpawn`) (`KismetMathLibrary.MakeTransform` _outlocation _outrotating (`KismetMathLibrary.Conv_DoubleToVector` (* _index_2 (`self.randomizescaleminimum`)))) false))))))